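; BP_Pawn is a player camera pawn that pans, zooms and rotates in yaw steps with smoothed motion.
; Axis and action inputs only update desired location, spring arm length and rotation, which BeginPlay seeds from the starting state.
; Tick interpolates the actor and SpringArm toward those targets.
; Panning follows the actor's forward and right vectors without delta-time scaling, while zoom is clamped to set limits.
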(event EventTick
  (params (DeltaSeconds :type Float%20%28single-precision%29))
  (bind _springarm (Variables|Default|GetSpringArm))
  ;[0 0 0] Set camera vector location and rotation based on desired X, Y, Zoom input, and rotation
  (Variables|/Script/Engine.SpringArmComponent|SetTargetArmLength _springarm (Math|Interpolation|FInterpTo (Variables|/Script/Engine.SpringArmComponent|GetTargetArmLength _springarm) (Variables|CameraControls|GetZoom_Desired) DeltaSeconds 2.0))
  (Transformation|SetActorLocation (Math|Interpolation|VInterpTo (Transformation|GetActorLocation) (Variables|CameraControls|GetLocation_Desired) DeltaSeconds 5.0) false false)
  (Transformation|SetActorRotation (Math|Interpolation|RInterpTo (Transformation|GetActorRotation) (Variables|CameraControls|GetRotation_Desired) DeltaSeconds 2.0)))

(event EventBeginPlay
  ;[0 0 0] Set default camera position based on player start location and spring arm length
  (Variables|CameraControls|SetLocation_Desired (Transformation|GetActorLocation))
  (Variables|CameraControls|SetZoom_Desired (Variables|/Script/Engine.SpringArmComponent|GetTargetArmLength (Variables|Default|GetSpringArm)))
  (Variables|CameraControls|SetRotation_Desired (Transformation|GetActorRotation)))

(event Input|ActionEvents|InputActionInputAction_Rotation_CW
  (params (Key :type Key%20Structure :default "None"))
  ;[0 0 0] Increment the rotation of the camera by the rotation step every time the inputaction rotation is called
  (:Pressed
    (Variables|CameraControls|SetRotation_Desired (Math|Rotator|CombineRotators (Variables|CameraControls|GetRotation_Desired) (Math|Rotator|MakeRotator 0.0 0.0 (Variables|CameraControls|GetRotation_Step))))))

(event Input|ActionEvents|InputActionInputAction_Rotation_CCW
  (params (Key :type Key%20Structure :default "None"))
  ;[0 0 0] Increment the rotation of the camera by the rotation step every time the inputaction rotation is called
  (:Pressed
    (Variables|CameraControls|SetRotation_Desired (Math|Rotator|CombineRotators (Variables|CameraControls|GetRotation_Desired) (Math|Rotator|MakeRotator 0.0 0.0 (* (Variables|CameraControls|GetRotation_Step) -1.0))))))

(event Input|AxisEvents|InputAxisInputAxis_Zoom
  (params (AxisValue :type Float%20%28single-precision%29))
  ;[0 0 0] Determine desired zoom using mouse scroll wheel
  (Variables|CameraControls|SetZoom_Desired (Math|Float|Clamp(Float) (+ (* AxisValue (Variables|Camera_Controls|GetZoom_Speed)) (Variables|CameraControls|GetZoom_Desired)) (Variables|CameraControls|GetZoom_Min) (Variables|CameraControls|GetZoom_Max))))

(event Input|AxisEvents|InputAxisInputAxis_Foward
  (params (AxisValue :type Float%20%28single-precision%29))
  ;[0 0 0] Controlling X Y movement
  (Variables|CameraControls|SetLocation_Desired (+ (Variables|CameraControls|GetLocation_Desired) (* (* AxisValue (Variables|CameraControls|GetCamera_Speed)) (Transformation|GetActorForwardVector)))))

(event Input|AxisEvents|InputAxisInputAxis_Right
  (params (AxisValue :type Float%20%28single-precision%29))
  ;[0 0 0] Controlling X Y movement
  (Variables|CameraControls|SetLocation_Desired (+ (Variables|CameraControls|GetLocation_Desired) (* (* AxisValue (Variables|CameraControls|GetCamera_Speed)) (Transformation|GetActorRightVector)))))

(fn ConstructionScript)