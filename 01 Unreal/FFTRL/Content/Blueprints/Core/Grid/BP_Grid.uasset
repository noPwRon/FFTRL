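; BP_Grid is a tile grid actor that builds its layout in the construction script from center, tile size, tile count and shape.
; SpawnGrid reads mesh, material and map dimensions from shape and size DataTables, then adds scaled instances to one InstancedStaticMesh.
; HeightRandomizer keeps border tiles flat and randomly offsets inner tiles by Intensity, using a clamped height multiplier carried from tile to tile.
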(event EventBeginPlay)

(event Collision|EventActorBeginOverlap
  (params (OtherActor :type Actor%20Object%20Reference)))

(event EventTick
  (params (DeltaSeconds :type Float%20%28single-precision%29)))

(fn ConstructionScript
  ;[0 0 0] Generate a new grid when the following properties are modified
  (CallFunction|SpawnGrid (Variables|Default|GetGridCenterLocation) (Variables|Default|GetGridTileSize) (Variables|Default|GetGridTileCount) (Variables|Default|GetGridShape)))

(fn SpawnGrid
  (params (CenterLocation :type Vector) (TileSize :type Vector :default "150.000000,150.000000,50.000000") (TileCount :type E_GridSize%20Enum :default "NewEnumerator0") (Shape :type E_GridShape%20Enum :default "NewEnumerator0"))
  (bind _returnvalue (CallFunction|GetCurrentShapeData))
  (bind _instancedstaticmesh (Variables|Default|GetInstancedStaticMesh))
  (bind (_mesh _meshmaterial) (Utilities|Struct|BreakS_GridShapeData _returnvalue))
  ;[0 0 0] Creating editable variables for the grid generation
  (Variables|Default|SetGridCenterLocation CenterLocation)
  (Variables|Default|SetGridTileSize TileSize)
  (Variables|Default|SetGridTileCount TileCount)
  (Variables|Default|SetGridShape Shape)
  ;[0 0 0] Loading static mesh and material based on grid shape
  (Components|StaticMesh|SetStaticMesh _instancedstaticmesh _mesh)
  (Rendering|Material|SetMaterial _instancedstaticmesh 0 _meshmaterial)
  ;[0 0 0] Get grid bottom left corner location
  (Variables|Default|SetGridBottomLeftCornerLocation (CallFunction|GetBottomLeftCornerLocation))
  (LocalVariables|SetMultiplier 1)
  (for _index (range 0 (- (Math|Float|Round (.x (.mapsize (CallFunction|GetCurrentCountData)))) 1))
    (LocalVariables|SetX _index)
    (for _index_2 (range 0 (- (Math|Float|Round (.y (.mapsize (CallFunction|GetCurrentCountData)))) 1))
      (LocalVariables|SetY _index_2)
      (Development|PrintString (Utilities|String|ToString(Integer) (LocalVariables|GetMultiplier)))
      (bind (_tiletransform _newmultiplier) (CallFunction|GetTileTransform (LocalVariables|GetMultiplier) (LocalVariables|GetX) (LocalVariables|GetY)))
      (LocalVariables|SetMultiplier _newmultiplier)
      (bind _output_get (LocalVariables|SetTileTransform (Math|Transform|MakeTransform _tiletransform "0, 0, 0" (/ (Variables|Default|GetGridTileSize) (Utilities|Struct|BreakS_GridShapeData (CallFunction|GetCurrentShapeData))))))
      (Components|InstancedStaticMesh|AddInstance (Variables|Default|GetInstancedStaticMesh) _output_get false))))

(fn GetCurrentShapeData
  (bind _gridshape (Variables|Default|GetGridShape))
  (bind _returnvalue (Utilities|String|EnumtoString _gridshape))
  (bind _returnvalue_2 (Utilities|GetDataTableRow "/Game/Blueprints/Core/Grid/Grid_Shape/DT_GridShapeData.DT_GridShapeData" (Utilities|String|StringToName _returnvalue))
    (:then
      (return _returnvalue_2))
    (:RowNotFound
      (Development|PrintString (Utilities|String|Append "Error: - Row not found - " _returnvalue) false true "(R=1.000000,G=0.017792,B=0.000000,A=1.000000)" 5.0))))

(fn GetCurrentCountData
  (bind _gridtilecount (Variables|Default|GetGridTileCount))
  (bind _returnvalue (Utilities|String|EnumtoString _gridtilecount))
  (bind _returnvalue_2 (Utilities|GetDataTableRow "/Game/Blueprints/Core/Grid/Grid_Shape/DT_GridSizeData.DT_GridSizeData" (Utilities|String|StringToName _returnvalue))
    (:then
      (return _returnvalue_2))
    (:RowNotFound
      (Development|PrintString (Utilities|String|Append "Error: - Row not found - " _returnvalue) false true "(R=1.000000,G=0.017792,B=0.000000,A=1.000000)" 5.0))))

(fn GetBottomLeftCornerLocation
  (return (- (Variables|Default|GetGridCenterLocation) (* (/ (Utilities|Struct|BreakS_GridSizeData (CallFunction|GetCurrentCountData)) 2.0) (Variables|Default|GetGridTileSize)))))

(fn HeightRandomizer
  (params (Intensity :type Float%20%28double-precision%29) (X :type Integer) (Y :type Integer) (TileHeight :type Float%20%28double-precision%29) (Multiplier :type Integer))
  (if (CallFunction|BorderCheck X Y)
    (return 0.0 0)
    (else
      (LocalVariables|SetRanGen (Math|Random|RandomFloatinRange -0.5 0.5))
      (LocalVariables|SetupDownVal (Math|Integer|SelectInt 1 -1 (>= (LocalVariables|GetRanGen) 0.0)))
      (if (> (Math|Float|Absolute(Float) (LocalVariables|GetRanGen)) (- 0.5 (* Intensity 0.5)))
        (return (* TileHeight Multiplier) (LocalVariables|GetupDownVal))
        (else
          (return 0.0 0))))))

(fn BorderCheck
  (params (X :type Integer) (Y :type Integer))
  (bind _returnvalue (CallFunction|GetCurrentCountData))
  (return (Math|Boolean|ORBoolean (== X 0) (== X (Class|KismetMathLibrary|Round64 (- (.x (.mapsize _returnvalue)) 1.0))) (== (Class|KismetMathLibrary|Round64 (- (.y (.mapsize _returnvalue)) 1.0)) Y) (== Y 0))))

(fn GetTileTransform
  (params (Multiplier :type Integer) (X :type Integer) (Y :type Integer))
  (bind _intensity (Variables|Default|GetIntensity))
  (bind _gridtilesize (Variables|Default|GetGridTileSize))
  (bind _returnvalue (Math|Float|Clamp(Float) _intensity))
  (bind _returnvalue_2 (Math|Conversions|ToFloat(Integer) X))
  (bind _returnvalue_3 (Math|Conversions|ToFloat(Integer) Y))
  (bind (_zlocation _multipliershift) (CallFunction|HeightRandomizer _returnvalue X Y 5e+01 Multiplier))
  (bind _returnvalue_4 (* _gridtilesize (Math|Vector|MakeVector _returnvalue_2 _returnvalue_3 0.0)))
  (return (+ (Variables|Default|GetGridBottomLeftCornerLocation) (Math|Vector|MakeVector (.x _returnvalue_4) (.y _returnvalue_4) _zlocation)) (Math|Integer|Clamp(Integer) (+ _multipliershift Multiplier) (Variables|Default|GetClampMin) (Variables|Default|GetClampMax))))